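; BP_Agent is an agent with Hunger, Sleep and Fun needs that decay over time and determine its most pressing need.
; Tick lowers all three by a shared DecreaseRate, clamps them between fixed bounds and prints them for debugging.
; A looping timer started on BeginPlay runs UpdateCurrentNeed, which sets the CurrentNeed enum to the lowest stat, favoring Hunger then Sleep on ties, and prints it.
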(event `self.ReceiveBeginPlay`
  (`KismetSystemLibrary.K2_SetTimer` null "UpdateCurrentNeed" 1.0 true))

(event `self.ReceiveTick`
  (params (DeltaSeconds :type "Float (single-precision)"))
  (set `self.Hunger` (`KismetMathLibrary.FClamp` (- (`self.Hunger`) (* DeltaSeconds (`self.DecreaseRate`))) 0.0 100.0))
  (set `self.Sleep` (`KismetMathLibrary.FClamp` (- (`self.Sleep`) (* DeltaSeconds (`self.DecreaseRate`))) 0.0 100.0))
  (set `self.Fun` (`KismetMathLibrary.FClamp` (- (`self.Fun`) (* DeltaSeconds (`self.DecreaseRate`))) 0.0 100.0))
  (`KismetSystemLibrary.PrintString` (`KismetTextLibrary.Conv_TextToString` (`|FormatText` "Hunger: {H} Sleep: {S} Fun: {F}" (`self.Hunger`) (`self.Sleep`) (`self.Fun`)))))

(fn `UpdateCurrentNeed`
  (if (`KismetMathLibrary.Conv_IntToBool` (`KismetMathLibrary.And_IntInt` (`KismetMathLibrary.Conv_BoolToInt` (<= (`self.Hunger`) (`self.Sleep`))) (`KismetMathLibrary.Conv_BoolToInt` (<= (`self.Hunger`) (`self.Fun`)))))
    (set `self.CurrentNeed` "NewEnumerator5")
    (elif (`KismetMathLibrary.Conv_IntToBool` (`KismetMathLibrary.And_IntInt` (`KismetMathLibrary.Conv_BoolToInt` (<= (`self.Sleep`) (`self.Hunger`))) (`KismetMathLibrary.Conv_BoolToInt` (<= (`self.Sleep`) (`self.Fun`)))))
      (set `self.CurrentNeed` "NewEnumerator6")
      (else
        (set `self.CurrentNeed` "NewEnumerator7"))))
  (`KismetSystemLibrary.PrintString` (`|GetEnumeratorNameAsString` (`self.CurrentNeed`)) true true (struct :`R` 1.0 :`G` 0.030652 :`A` 1.0) 1.0))

(fn `UserConstructionScript`)